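; BP_Zombie is an enemy character that chases and damages the first-person player.
; On spawn it randomizes mesh scale, facing and walk speed for variety.
; PawnSensing sightings start an AI MoveTo toward the player, applying damage when it succeeds.
; Kill stops AI logic, ragdolls the mesh, then after a short delay fires OnKilled and destroys the actor.
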(event `self.ReceiveBeginPlay`
  (bind _returnvalue (`KismetMathLibrary.RandomFloatInRange` 0.9 1.1))
  (`SceneComponent.SetWorldScale3D` (`self.Mesh`) (`KismetMathLibrary.MakeVector` _returnvalue _returnvalue _returnvalue))
  (`self.K2_SetActorRotation` (`KismetMathLibrary.MakeRotator` 0.0 0.0 (`KismetMathLibrary.RandomFloatInRange` 0.0 360.0)))
  (set `CharacterMovementComponent.MaxWalkSpeed` (`KismetMathLibrary.RandomFloatInRange` 450.0 700.0) (`self.CharacterMovement`)))

(event `Kill`
  (bind _mesh (`self.Mesh`))
  (`BrainComponent.StopLogic` (`AIController.BrainComponent` (`AIBlueprintHelperLibrary.GetAIController` self)) "")
  (`PrimitiveComponent.SetCollisionProfileName` _mesh "Ragdoll" true)
  (`PrimitiveComponent.SetSimulatePhysics` _mesh true)
  (`PrimitiveComponent.SetCollisionProfileName` (`self.CapsuleComponent`) "NoCollision" true)
  (`KismetSystemLibrary.Delay` 1.0)
  (`self.OnKilled` self)
  (`self.K2_DestroyActor`))

(event `self.PawnSensing.OnSeePawn`
  (params (Pawn :type "Pawn Object Reference"))
  (bind _asfirst_person_character (cast `/Game/FirstPersonBP/Blueprints/FirstPersonCharacter` Pawn))
  (`|AIMoveTo` self (0.0 0.0 0.0) _asfirst_person_character
    (:`OnSuccess`
      (`GameplayStatics.ApplyDamage` _asfirst_person_character (`self.Damage`)))))

(fn `UserConstructionScript`)